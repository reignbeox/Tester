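; BP_Shooter is a projectile launcher that spawns BP_Projectile at a spawn point, though nothing in its graph starts the firing timeline.
; Timeline updates are gated by CanShoot and a delay, with each shot pushing the projectile's Ball by a force from the Arrow's forward X and ShootingPower.
; Each shot also passes a hit effect to the projectile, spawns a muzzle flash and attaches a trail.
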(fn `UserConstructionScript`)