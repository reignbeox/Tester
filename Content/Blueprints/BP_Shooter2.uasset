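; BP_Shooter2 is a projectile shooter, though nothing in its graph starts the firing timeline, so it never fires as written.
; The timeline update would spawn a scaled BP_Projectile, gated by CanShoot and a delay.
; It pushes the ball using only the Arrow forward vector's X component, scaled by ShootingPower.
; It also passes on a hit effect and spawns muzzle flash and trail particles.
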(fn `UserConstructionScript`)