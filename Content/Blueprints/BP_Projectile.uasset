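; Projectile actor with a physics ball and collision volume that expires after a set lifespan or shortly after hitting something.
; On hit it hides the ball, flags itself dead, stops physics on both components and destroys itself after a brief delay.
; A DoOnce gate spawns a single Niagara impact effect at the hit location, oriented along the rotated hit normal.
; A BeginTrails call is present but never runs.
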(event `self.ReceiveBeginPlay`
  ;[0 0 0] Set Default Lifetime
  (set `self.IsDead` false)
  (`self.SetLifeSpan` 10.0))

(event `self.ReceiveHit`
  (params (MyComp :type "PrimitiveComponent Object Reference") (Other :type "Actor Object Reference") (OtherComp :type "PrimitiveComponent Object Reference") (bSelfMoved :type Boolean) (HitLocation :type "Vector Structure") (HitNormal :type "Vector Structure") (NormalImpulse :type "Vector Structure") (Hit :type "HitResult Structure (by ref)"))
  ;[0 0 0] Destroy Ball on Hit
  (bind _output_get (set `self.Hit Location` HitLocation))
  (`|ExecutionSequence`
    (:`then_0`
      (`SceneComponent.SetVisibility` (`self.Ball`) false false)
      (set `self.IsDead` true)
      (`PrimitiveComponent.SetSimulatePhysics` (`self.Ball`) false)
      (`PrimitiveComponent.SetSimulatePhysics` (`self.Collision Volume`) false)
      (`KismetSystemLibrary.Delay` 0.5)
      (`self.K2_DestroyActor`))
    (:`then_1`
      ;[0 0 0] Spawn Default Particle
      (`/Engine/EditorBlueprintResources/StandardMacros.DoOnce` false
        (:`Completed`
          (`NiagaraFunctionLibrary.SpawnSystemAtLocation` (`self.Hit PS`) _output_get (`KismetMathLibrary.Conv_VectorToRotator` (`KismetMathLibrary.GreaterGreater_VectorRotator` HitNormal (`self.Rotate By`)))))))))

(fn `UserConstructionScript`)